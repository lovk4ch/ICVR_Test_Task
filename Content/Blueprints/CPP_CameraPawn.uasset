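; Camera pawn that continuously travels along its own spline, restarting from the beginning each time it finishes.
; On BeginPlay it caches the spline length and plays a timeline that maps to distance along the spline.
; Each update broadcasts BeforeCameraMoved with the next local location, then moves the camera, following spline yaw and roll at a fixed downward pitch.
; A getter exposes the camera's world location.
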(event EventBeginPlay
  (Utilities|FlowControl|Sequence
    (:then_0
      (Variables|Default|SetLength (Spline|GetSplineLength (Variables|Default|GetSpline))))
    (:then_1
      (bind _position (Timeline|SplineMovement PlayFromStart)
        (:Update
          (Default|CallBeforeCameraMoved (Spline|GetLocationatDistanceAlongSpline (Variables|Default|GetSpline) (* _position (Variables|Default|GetLength)) "Local"))
          (Transformation|SetRelativeLocation (Variables|Default|GetCamera) (Spline|GetLocationatDistanceAlongSpline (Variables|Default|GetSpline) (* _position (Variables|Default|GetLength)) "Local") false false)
          (Transformation|SetRelativeRotation (Variables|Default|GetCamera) (Math|Rotator|MakeRotator (.roll (Spline|GetRotationatDistanceAlongSpline (Variables|Default|GetSpline) (* _position (Variables|Default|GetLength)) "Local")) -15.0 (.yaw (Spline|GetRotationatDistanceAlongSpline (Variables|Default|GetSpline) (* _position (Variables|Default|GetLength)) "Local"))) true false))
        (:Finished
          (Timeline|SplineMovement PlayFromStart))))))

(fn ConstructionScript)

(fn GetCameraWorldLocation
  (return (Transformation|GetWorldLocation (Variables|Default|GetCamera))))
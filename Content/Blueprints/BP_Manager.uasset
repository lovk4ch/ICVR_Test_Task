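; BP_Manager is a manager that spawns thousands of randomly placed CPP_Cube actors and binds to the camera pawn's before-move event.
; PredictCubeColors recolors recently rendered cubes by distance to a given location and prints their count.
; GetColorByDistance uses two capped distance tiers, blue then yellow, with red as fallback; per-pass counters fill the caps in array order, not nearest-first.
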(event EventBeginPlay
  (Utilities|FlowControl|Sequence
    (:then_0
      (bind _ascpp_camera_pawn (Utilities|Casting|CastToCPP_CameraPawn (Game|Player|GetPlayerPawn 0)))
      (EventDispatchers|BindEventtoBeforeCameraMoved _ascpp_camera_pawn (EventDispatchers|CreateEvent :!event PredictCubeColors)))
    (:then_1
      (for _index (range 0 2999)
        (bind _returnvalue (Game|SpawnActorfromClass "/Game/Blueprints/CPP_Cube.CPP_Cube_C" (Math|Transform|MakeTransform (Math|Vector|MakeVector (Math|Random|RandomFloatinRange -1.5e+04 1.5e+04) (Math|Random|RandomFloatinRange -1.5e+04 1.5e+04) (Math|Random|RandomFloatinRange -25.0 1175.0)) "0, 0, 0" "1,1,1") "Undefined" 0 0))
        (Utilities|Array|Add (Variables|Default|GetCubes) _returnvalue)))))

(fn ConstructionScript)

(fn PredictCubeColors
  (params (Location :type Vector))
  (Variables|Default|SetRenderedCubesCount 0)
  (Variables|R0|SetL0_Current 0)
  (Variables|R1|SetL1_Current 0)
  (for _array_element (Variables|Default|GetCubes)
    (if (Class|Actor|WasRecentlyRendered _array_element 0.1)
      (bind _color (CallFunction|GetColorbyDistance (Math|Vector|Distance(Vector) (Transformation|GetWorldLocation (Variables|/Script/ICVR_Test_Task.Cube|GetRoot _array_element)) Location)))
      (Default|SetColor _array_element "Color" _color)
      (Math|Integer|IncrementInt (Variables|Default|GetRenderedCubesCount))))
  (Development|PrintString (Utilities|String|Append "Total cubes in FOV: " (Utilities|String|ToString(Integer) (Variables|Default|GetRenderedCubesCount))) true true "(R=0.000000,G=0.660000,B=1.000000,A=1.000000)" 0.0))

(fn GetColorbyDistance
  (params (Distance :type Float%20%28single-precision%29))
  (if (< (Variables|R0|GetL0_Current) (Variables|R0|GetL0))
    (if (< Distance (Variables|R0|GetR0))
      (Math|Integer|IncrementInt (Variables|R0|GetL0_Current)
        (:%20%20
          (return "(R=0.000000,G=0.000000,B=1.000000,A=1.000000)")))
      (else
        _)))
  (if (< (Variables|R1|GetL1_Current) (Variables|R1|GetL1))
    (if (< Distance (Variables|R1|GetR1))
      (Math|Integer|IncrementInt (Variables|R1|GetL1_Current)
        (:%20%20
          (return "(R=1.000000,G=1.000000,B=0.000000,A=1.000000)")))
      (else
        _)))
  (return "(R=1.000000,G=0.000000,B=0.000000,A=1.000000)"))
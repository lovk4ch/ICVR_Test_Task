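; Manager Blueprint that spawns a large grid of BP_Cube actors and colors them in distance tiers around the camera.
; It binds to the CameraPawn's before-move event, and PredictCubeColors recolors recently rendered cubes using the camera's next location.
; GetColorByDistance assigns blue, yellow or red by radius, with the first two tiers capped by count in array order rather than nearest first.
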(event EventBeginPlay
  (Utilities|FlowControl|Sequence
    (:then_0
      (bind _ascamera_pawn (Utilities|Casting|CastToCameraPawn (Game|Player|GetPlayerPawn 0)))
      (bind _output_get (Variables|Default|SetCameraPawn _ascamera_pawn))
      (EventDispatchers|BindEventtoBeforeCameraMoved _output_get (EventDispatchers|CreateEvent :!event PredictCubeColors)))
    (:then_1
      (for _index (range 0 49)
        (for _index_2 (range 0 99)
          (bind _returnvalue (Game|SpawnActorfromClass "/Game/BP_Cube.BP_Cube_C" (Math|Transform|MakeTransform (+ (Math|Vector|MakeVector (+ (* _index -2.5e+02) (* (/ _index 10) -1e+03)) (* _index_2 2.5e+02) 0.0) (Math|Vector|MakeVector 5e+03 -5e+03 2e+01)) "0, 0, 0" "1,1,1") "Undefined" 0 0))
          (Utilities|Array|Add (Variables|Default|GetCubes) _returnvalue))))))

(fn ConstructionScript)

(fn PredictCubeColors
  (params (Location :type Vector))
  (Variables|Default|SetRenderedCubesCount 0)
  (Variables|R0|SetL0_Current 0)
  (Variables|R1|SetL1_Current 0)
  (LocalVariables|SetCameraNextLocation Location)
  (for _array_element (Variables|Default|GetCubes)
    (if (Class|Actor|WasRecentlyRendered _array_element 0.1)
      (bind _color (CallFunction|GetColorbyDistance (Math|Vector|Distance(Vector) (Transformation|GetWorldLocation (Variables|/Game/BP_Cube.BP_Cube_C|GetDefaultSceneRoot _array_element)) (LocalVariables|GetCameraNextLocation))))
      (Default|SetColor _array_element _color)
      (Math|Integer|IncrementInt (Variables|Default|GetRenderedCubesCount))))
  (Development|PrintString (Utilities|String|Append "Total cubes in FOV: " (Utilities|String|ToString(Integer) (Variables|Default|GetRenderedCubesCount))) true true "(R=0.000000,G=0.660000,B=1.000000,A=1.000000)" 0.0))

(fn GetColorbyDistance
  (params (Distance :type Float%20%28single-precision%29))
  (if (< (Variables|R0|GetL0_Current) (Variables|R0|GetL0))
    (if (< Distance (Variables|R0|GetR0))
      (Math|Integer|IncrementInt (Variables|R0|GetL0_Current)
        (:%20%20
          (return "(R=0.000000,G=0.000000,B=1.000000,A=1.000000)")))
      (else
        _)))
  (if (< (Variables|R1|GetL1_Current) (Variables|R1|GetL1))
    (if (< Distance (Variables|R1|GetR1))
      (Math|Integer|IncrementInt (Variables|R1|GetL1_Current)
        (:%20%20
          (return "(R=1.000000,G=1.000000,B=0.000000,A=1.000000)")))
      (else
        _)))
  (return "(R=1.000000,G=0.000000,B=0.000000,A=1.000000)"))